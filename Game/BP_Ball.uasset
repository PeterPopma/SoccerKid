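; Football actor that the player picks up on contact and dribbles.
; A hit from a BP_ThirdPersonCharacter without a ball registers itself on that character, then disables its physics and collision.
; While stuck, Tick teleports it to a lowered point ahead of player 0, whichever character hit it, and fakes rolling from that player's speed and right vector.
; A timer repeats a 2D dribble sound while the player moves.
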(event Collision|EventHit
  (params (MyComp :type Primitive%20Component%20Object%20Reference) (Other :type Actor%20Object%20Reference) (OtherComp :type Primitive%20Component%20Object%20Reference) (bSelfMoved :type Boolean) (HitLocation :type Vector :default "0, 0, 0") (HitNormal :type Vector :default "0, 0, 0") (NormalImpulse :type Vector :default "0, 0, 0") (Hit :type Hit%20Result%20Structure%20%28by%20ref%29))
  ;[1 1 1] Ball hit (by player)
  (bind _asbp_third_person_character (Utilities|Casting|CastToBP_ThirdPersonCharacter Other))
  (if (not (Variables|/Game/ThirdPerson/Blueprints/BP_ThirdPersonCharacter.BP_ThirdPersonCharacter_C|GetHasBall _asbp_third_person_character))
    (Variables|Default|SetUsedByPlayer true)
    (Variables|/Game/ThirdPerson/Blueprints/BP_ThirdPersonCharacter.BP_ThirdPersonCharacter_C|SetHasBall _asbp_third_person_character true)
    (Variables|/Game/ThirdPerson/Blueprints/BP_ThirdPersonCharacter.BP_ThirdPersonCharacter_C|SetBall _asbp_third_person_character self)
    (Variables|Default|SetStickToPlayer true)
    (Physics|SetSimulatePhysics (Variables|Default|Getfootball_ball_FBX) false)
    (Collision|SetActorEnableCollision false)))

(event EventTick
  (params (DeltaSeconds :type Float%20%28single-precision%29))
  (bind _returnvalue (Game|GetPlayerCharacter 0))
  (bind _returnvalue_2 (Transformation|GetActorLocation _returnvalue))
  (bind _returnvalue_3 (Transformation|GetActorForwardVector _returnvalue))
  (bind _returnvalue_4 (Transformation|GetVelocity _returnvalue))
  (bind _returnvalue_5 (Transformation|GetActorRightVector _returnvalue))
  (bind _returnvalue_6 (Math|Vector|VectorLength _returnvalue_4))
  (bind _returnvalue_7 (Math|Vector|Normalize _returnvalue_5))
  (bind _returnvalue_8 (* _returnvalue_3 1e+02))
  (bind _returnvalue_9 (* _returnvalue_6 -0.02))
  (bind _returnvalue_10 (+ _returnvalue_8 _returnvalue_2))
  (bind (_x _y _z) (Math|Vector|BreakVector _returnvalue_10))
  (bind _returnvalue_11 (* _returnvalue_7 _returnvalue_9))
  (bind (_x_2 _y_2) (Math|Vector|BreakVector _returnvalue_11))
  ;[1 1 1] Stick ball to player
  (if (Variables|Default|GetStickToPlayer)
    (Transformation|SetActorLocation (Math|Vector|MakeVector _x _y (- _z 6e+01)) false true)
    (Class|Actor|AddActorWorldRotation (Math|Rotator|MakeRotator _x_2 _y_2 0.0))
    (if (> (Math|Vector|VectorLength (Transformation|GetVelocity (Game|Player|GetPlayerPawn 0))) 0.0)
      (bind _output_get (Variables|Default|SetTimeLastSoundPlay (+ DeltaSeconds (Variables|Default|GetTimeLastSoundPlay))))
      (if (> _output_get 0.8)
        (Variables|Default|SetTimeLastSoundPlay 0.0)
        (Audio|PlaySound2D "/Game/Sounds/soccerballrun.soccerballrun" 1.0 1.0 0.0 0 0)))))

(fn ConstructionScript)