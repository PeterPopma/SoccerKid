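; BP_Target is a one-shot target that scores when hit by a player-used BP_Ball.
; A hit launches the Peter component with physics, impulse and torque, plus sound and explosion effects.
; Points equal the distance from the character's ShootLocation to the target, and are added to the game mode's score.
; Tick projects the hit position to screen space, floating a UI_HitPoints widget upward while fading it out, then removes it.
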(event EventTick
  (params (DeltaSeconds :type Float%20%28single-precision%29))
  (bind _returnvalue (Game|GetPlayerController 0))
  (bind _hitposition (Variables|Default|GetHitPosition))
  (bind _screenposition (Class|GameplayStatics|ProjectWorldtoScreen _returnvalue _hitposition false))
  (bind (_x _y) (Math|Vector2D|BreakVector2D _screenposition))
  ;[1 1 1] Score floating above target
  (if (Variables|Default|GetHitAnimRunning)
    (Variables|Default|SetYOffset (- (Variables|Default|GetYOffset) (* DeltaSeconds 5e+02)))
    (Class|UserWidget|SetPositioninViewport (stale Collision|EventHit _returnvalue) (Math|Vector2D|MakeVector2D _x (+ (Variables|Default|GetYOffset) _y)) true)
    ;[1 1 1] Score fade out
    (Widget|SetRenderOpacity (stale Collision|EventHit _returnvalue) (- (Variables|Default|GetOne) (/ (Variables|Default|GetYOffset) -4e+02)))
    ;[1 1 1] Animation finished
    (if (< (Variables|Default|GetYOffset) -4e+02)
      (Widget|RemovefromParent (stale Collision|EventHit _returnvalue))
      (Variables|Default|SetHitAnimRunning false))))

(event Collision|EventHit
  (params (MyComp :type Primitive%20Component%20Object%20Reference) (Other :type Actor%20Object%20Reference) (OtherComp :type Primitive%20Component%20Object%20Reference) (bSelfMoved :type Boolean) (HitLocation :type Vector :default "0, 0, 0") (HitNormal :type Vector :default "0, 0, 0") (NormalImpulse :type Vector :default "0, 0, 0") (Hit :type Hit%20Result%20Structure%20%28by%20ref%29))
  (bind _peter (Variables|Default|GetPeter))
  (if (not (Variables|Default|GetHas%20Been%20Hit))
    (bind _asbp_ball (Utilities|Casting|CastToBP_Ball Other))
    (if (Variables|/Game/Game/BP_Ball.BP_Ball_C|GetUsedByPlayer _asbp_ball)
      (Variables|Default|SetHas%20Been%20Hit true)
      (Variables|Default|SetHitAnimRunning true)
      (Variables|Default|SetHitPosition HitLocation)
      ;[1 1 1] Hit effects
      (Physics|SetSimulatePhysics _peter true)
      (Physics|AddImpulse _peter (* (.ImpactNormal (Collision|BreakHitResult Hit)) 1.2e+03) "None" true)
      (Class|PrimitiveComponent|AddTorqueinRadians _peter (* (Math|Vector|GetRightVector _peter) 7e+02) "None" true)
      (Audio|PlaySoundatLocation "/Game/Sounds/targethit.targethit" HitLocation "0, 0, 0" 1.0 1.0 0.0 0 0 0 0)
      (Effects|SpawnEmitteratLocation "/Game/StarterContent/Particles/P_Explosion.P_Explosion" HitLocation)
      (bind _asbp_third_person_character (Utilities|Casting|CastToBP_ThirdPersonCharacter (Game|GetPlayerCharacter 0)))
      (bind _asbp_third_person_game_mode (Utilities|Casting|CastToBP_ThirdPersonGameMode (Game|GetGameMode)))
      ;[1 1 1] Calculate score
      (bind _output_get (Variables|Default|SetHitPoints (Math|Float|Round (Math|Vector|VectorLength (- (Variables|/Game/ThirdPerson/Blueprints/BP_ThirdPersonCharacter.BP_ThirdPersonCharacter_C|GetShootLocation _asbp_third_person_character) (Transformation|GetActorLocation))))))
      ;[1 1 1] Set score text
      (Variables|/Game/ThirdPerson/Blueprints/BP_ThirdPersonGameMode.BP_ThirdPersonGameMode_C|SetScore _asbp_third_person_game_mode (+ (Variables|/Game/ThirdPerson/Blueprints/BP_ThirdPersonGameMode.BP_ThirdPersonGameMode_C|GetScore _asbp_third_person_game_mode) _output_get))
      (Default|UpdateScore _asbp_third_person_game_mode)
      (bind _returnvalue (UserInterface|CreateWidget "/Game/Game/UI_HitPoints.UI_HitPoints_C"))
      (UserInterface|Viewport|AddtoViewport _returnvalue 0)
      (Rendering|Components|TextRender|SetText (Variables|/Game/Game/UI_HitPoints.UI_HitPoints_C|GetHitPoints _returnvalue) (Utilities|Text|ToText(Integer) _output_get false false)))))

(fn ConstructionScript)